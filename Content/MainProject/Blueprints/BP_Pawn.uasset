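; AR player pawn for placing and sizing Christmas tree models on detected real-world surfaces.
; BeginPlay loads or creates the save and stores it in Global_Var; Tick creates the panel UI, starts the AR session and moves a reticle via screen-centre AR traces, prompting when none hits.
; Touch swaps the reticle for the selected tree or removes it.
; A slider rescales the tree through per-species height tables and reports its size.
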(event `self.ReceiveBeginPlay`
  ;[1 1 1] Start
  (bind (_savegame _bsuccess) (`AsyncActionHandleSaveGame.AsyncLoadGameFromSlot` (`self.SaveNameSlot`) (`self.UserIndex`))
    (:`Completed`
      (if _bsuccess
        (bind _asbp_save_game (cast `/Game/MainProject/Blueprints/BP_SaveGame` _savegame))
        (bind _asglobal_var (cast `/Game/MainProject/Blueprints/Global_Var` (`GameplayStatics.GetGameInstance`)))
        (set `/Game/MainProject/Blueprints/Global_Var.SaveGameObject` _asbp_save_game _asglobal_var)
        (bind _asglobal_var_2 (cast `/Game/MainProject/Blueprints/Global_Var` (`GameplayStatics.GetGameInstance`)))
        (set `/Game/MainProject/Blueprints/Global_Var.FirstWidget` true _asglobal_var_2)
        (else
          (bind _returnvalue (`GameplayStatics.CreateSaveGameObject` "/Game/MainProject/Blueprints/BP_SaveGame.BP_SaveGame_C"))
          (`AsyncActionHandleSaveGame.AsyncSaveGameToSlot` _returnvalue (`self.SaveNameSlot`) (`self.UserIndex`)
            (:`Completed`
              (bind _asglobal_var_3 (cast `/Game/MainProject/Blueprints/Global_Var` (`GameplayStatics.GetGameInstance`)))
              (set `/Game/MainProject/Blueprints/Global_Var.SaveGameObject` _returnvalue _asglobal_var_3)
              (bind _returnvalue_2 (`|CreateWidget` "/Game/MainProject/Widgets/FirstLaunchWidget.FirstLaunchWidget_C"))
              (`UserWidget.AddToViewport` _returnvalue_2 0)))))
      (bind _newparam (`self.GetMiddleOfScreen`))
      (set `self.Vec_Coord` _newparam)
      (set `self.Chek_touch` false)
      (set `self.Chek_Circle` true))))

(event `self.ReceiveTick`
  (params (DeltaSeconds :type "Float (single-precision)"))
  (bind _chek_circle (`self.Chek_Circle`))
  ;[1 1 1] Replace circle
  (bind _asglobal_var (cast `/Game/MainProject/Blueprints/Global_Var` (`GameplayStatics.GetGameInstance`)))
  (if (`/Game/MainProject/Blueprints/Global_Var.FirstWidget` _asglobal_var)
    (if (not (`self.First`))
      (bind _returnvalue (`|CreateWidget` "/Game/MainProject/Widgets/PanelWidget.PanelWidget_C"))
      (`UserWidget.AddToViewport` _returnvalue 0)
      (set `/Game/MainProject/Widgets/PanelWidget.CurrentWidget` _returnvalue _returnvalue)
      (set `self.PanelWidget` _returnvalue)
      (set `self.First` true)
      (`ARBlueprintLibrary.StartARSession` "/Game/MainProject/Blueprints/D_SessionConfig.D_SessionConfig"))
    (bind _asglobal_var_2 (cast `/Game/MainProject/Blueprints/Global_Var` (`GameplayStatics.GetGameInstance`)))
    (if (`/Game/MainProject/Blueprints/Global_Var.Opened` _asglobal_var_2)
      (if (`self.Chek_touch`)
        (`self.K2_DestroyActor` (`self.Tree_addr`))
        (set `self.Chek_touch` false)
        (set `self.Chek_Circle` true :!label _label)
        (elif (not (`self.Chek_Circle`))
          (`self.K2_DestroyActor` (`self.Circle_addr`))
          (goto _label)))
      (elif _chek_circle
        (bind (_actor_addr _error) (`self.My_Spawn` "/Game/MainProject/Blueprints/BP_Circle.BP_Circle_C"))
        (if (not _chek_circle)
          (`self.K2_DestroyActor` (`self.Circle_addr`)))
        (set `self.Chek_Circle` _error)
        (elif (`self.Chek_touch`)
          (bind _asglobal_var_3 (cast `/Game/MainProject/Blueprints/Global_Var` (`GameplayStatics.GetGameInstance`)))
          (`self.My_Resize` (`self.Tree_addr`) (`/Game/MainProject/Blueprints/Global_Var.Size Value of Elka Slider` _asglobal_var_3))
          (else
            (`self.My_Replace` (`self.Circle_addr`))))))))

(event `InputTouch`
  (params (Location :type "Vector Structure") (FingerIndex :type "ETouchIndex Enum"))
  (bind _circle_addr (`self.Circle_addr`))
  (bind _panelwidget (`self.PanelWidget`))
  (bind _panelwidget_2 (`self.PanelWidget`))
  (bind _panelwidget_3 (`self.PanelWidget`))
  ;[1 1 1] Spawn and destroy tree
  (:`Pressed`
    (if (`self.Chek_Circle`)
      _
      (elif (`self.Chek_touch`)
        (set `self.Chek_touch` false)
        (`self.K2_DestroyActor` (`self.Tree_addr`))
        (set `self.Chek_Circle` true)
        (`UserWidget.PlayAnimationReverse` _panelwidget_2 (`/Game/MainProject/Widgets/PanelWidget.ShowSlider` _panelwidget_2) 1.0 false)
        (set `/Game/MainProject/Widgets/PanelWidget.SliderObject` false _panelwidget_2)
        (else
          (bind _asglobal_var (cast `/Game/MainProject/Blueprints/Global_Var` (`GameplayStatics.GetGameInstance`)))
          (bind _number_of_elka (`/Game/MainProject/Blueprints/Global_Var.Number of Elka` _asglobal_var))
          (`/Engine/EditorBlueprintResources/StandardMacros.CompareInt` _number_of_elka
            (:`>`
              (set `self.Chek_touch` true)
              (bind _output_get (set `self.Circle Transform` (`self.GetTransform` _circle_addr)))
              (`self.K2_DestroyActor` _circle_addr)
              (bind _returnvalue (`|SpawnActorFromClass` (`|GetArrayItem` (`|MakeArray` "/Game/MainProject/Blueprints/BP_Circle.BP_Circle_C" "/Game/MainProject/Blueprints/Elki/BP_DutchElka.BP_DutchElka_C" "/Game/MainProject/Blueprints/Elki/BP_ElkaPot.BP_ElkaPot_C" "/Game/MainProject/Blueprints/Elki/BP_PihtaFraseri.BP_PihtaFraseri_C" "/Game/MainProject/Blueprints/Elki/BP_RusElka.BP_RusElka_C" "/Game/MainProject/Blueprints/Elki/BP_RusSosna.BP_RusSosna_C" :!type "Actor Class Reference") _number_of_elka) _output_get "Undefined" "OverrideRootScale" null null))
              (set `self.Tree_addr` _returnvalue)
              (`UserWidget.PlayAnimationForward` _panelwidget (`/Game/MainProject/Widgets/PanelWidget.ShowSlider` _panelwidget) 1.0 false)
              (set `/Game/MainProject/Widgets/PanelWidget.SliderObject` true _panelwidget))
            (:`==`
              (`UserWidget.PlayAnimationForward` _panelwidget_3 (`/Game/MainProject/Widgets/PanelWidget.Warn` _panelwidget_3) 1.0 false))))))))

(fn `Delay`
  (params (Value :type Integer))
  (returns (Finish :type Boolean))
  (bind _count (`self.Count`))
  (`/Engine/EditorBlueprintResources/StandardMacros.CompareInt` Value _count
    (:`>`
      (set `self.Error1` true))
    (:`==`
      (`/Engine/EditorBlueprintResources/StandardMacros.IncrementInt` _count :!label _label
        (:`  `
          (set `self.Error1` false))))
    (:`<`
      (goto _label)))
  (return (`self.Error1`)))

(fn `GetMiddleOfScreen`
  (returns (NewParam :type "Vector2D Structure"))
  (bind _returnvalue (`GameUserSettings.GetGameUserSettings`))
  (bind (_x _y) (break `IntPoint` (`GameUserSettings.GetScreenResolution` _returnvalue)))
  (return (`KismetMathLibrary.MakeVector2D` (`KismetMathLibrary.Conv_IntToDouble` (/ _x 2)) (`KismetMathLibrary.Conv_IntToDouble` (/ _y 2)))))

(fn `My_Replace`
  (params (Actor_addr :type "Actor Object Reference"))
  (returns (Error :type Boolean))
  (set `self.Error` false)
  (bind (_outhit _returnvalue) (`self.WorldHitTest` (`self.Vec_Coord`)))
  (if _returnvalue
    (set `self.Error` true :!label _label)
    (`self.K2_DestroyActor` (`self.Circle_addr`))
    (set `self.Chek_Circle` true)
    (else
      (bind _returnvalue_2 (`ARBlueprintLibrary.LineTraceTrackedObjects` (`self.Vec_Coord`) false false))
      (`/Engine/EditorBlueprintResources/StandardMacros.CompareInt` (`KismetArrayLibrary.Array_Length` _returnvalue_2)
        (:`>`
          (`Widget.RemoveFromParent` (`self.Phone_addrNew`))
          (`self.K2_SetActorTransform` Actor_addr (`ARTraceResultLibrary.GetLocalToWorldTransform` (`|GetArrayItem` _returnvalue_2)) false true))
        (:`==`
          (goto _label))
        (:`<`
          (goto _label)))))
  (return (`self.Error`)))

(fn `My_Resize`
  (params (Actor :type "Actor Object Reference") (ScaleVector :type "Float (double-precision)"))
  (returns (NewParam :type "Float (double-precision)"))
  (bind _asglobal_var (cast `/Game/MainProject/Blueprints/Global_Var` (`GameplayStatics.GetGameInstance`)))
  (bind _asglobal_var_2 (cast `/Game/MainProject/Blueprints/Global_Var` (`GameplayStatics.GetGameInstance`)))
  (bind _number_of_elka (`/Game/MainProject/Blueprints/Global_Var.Number of Elka` _asglobal_var))
  (bind _returnvalue (+ (`|GetArrayItem` (`|MakeArray` 0.0 0.75 0.6 1.0 0.75 1.0 :!type "Float (single-precision)") _number_of_elka) (* (`|GetArrayItem` (`|MakeArray` 0.0 4.25 0.6 1.0 7.25 2.0 :!type "Float (single-precision)") _number_of_elka) ScaleVector)))
  (bind _output_get (set `/Game/MainProject/Blueprints/Global_Var.Size of Elka` _returnvalue _asglobal_var_2))
  (`/Game/MainProject/Widgets/PanelWidget.SetRealSizeOfElka` (`self.PanelWidget`) _output_get)
  (bind _returnvalue_2 (/ _returnvalue (`|GetArrayItem` (`|MakeArray` 0.0 1.63 1.47 1.4 1.69 2.46 :!type "Float (single-precision)") _number_of_elka)))
  (`self.K2_SetActorTransform` Actor (`KismetMathLibrary.MakeTransform` (`self.K2_GetActorLocation` Actor) (`self.K2_GetActorRotation` Actor) (`KismetMathLibrary.MakeVector` _returnvalue_2 _returnvalue_2 _returnvalue_2)) false false)
  (return _returnvalue_2))

(fn `My_Spawn`
  (params (Actor :type "Actor Class Reference"))
  (returns (Actor_addr :type "Actor Object Reference") (Error :type Boolean))
  (set `self.Error` false)
  (bind (_outhit _returnvalue) (`self.WorldHitTest` (`self.Vec_Coord`)))
  (if _returnvalue
    (set `self.Error` true :!label _label)
    (if (not (`self.error_spawn_circle`))
      (bind _returnvalue_2 (`|CreateWidget` "/Game/MainProject/Widgets/PhonePlaneWidget.PhonePlaneWidget_C"))
      (set `self.Phone_addrNew` _returnvalue_2)
      (`UserWidget.AddToViewport` _returnvalue_2 -1)
      (set `self.error_spawn_circle` true)
      (return null (`self.Error`)))
    (else
      (bind _returnvalue_3 (`ARBlueprintLibrary.LineTraceTrackedObjects` (`self.Vec_Coord`) false false))
      (`/Engine/EditorBlueprintResources/StandardMacros.CompareInt` (`KismetArrayLibrary.Array_Length` _returnvalue_3)
        (:`>`
          (bind _finish (`self.Delay` 150))
          (if _finish
            (set `self.Count` 0)
            (`Widget.RemoveFromParent` (`self.Phone_addrNew`))
            (bind _returnvalue_4 (`|SpawnActorFromClass` Actor (`ARTraceResultLibrary.GetLocalToWorldTransform` (`|GetArrayItem` _returnvalue_3)) "AlwaysSpawn" "OverrideRootScale" null null))
            (set `self.Circle_addr` _returnvalue_4)
            (set `self.error_spawn_circle` false)
            (return null (`self.Error`))
            (else
              (goto _label))))
        (:`==`
          (goto _label))
        (:`<`
          (goto _label))))))

(fn `UserConstructionScript`)

(fn `WorldHitTest`
  (params (ScreenPosition :type "Vector2D Structure (by ref)"))
  (returns (OutHit :type "HitResult Structure") (ReturnValue :type Boolean))
  (bind (_worldposition _worlddirection) (`GameplayStatics.DeprojectScreenToWorld` (`GameplayStatics.GetPlayerController` 0) ScreenPosition))
  (bind (_outhit _returnvalue) (`KismetSystemLibrary.LineTraceSingleForObjects` _worldposition (+ _worldposition (+ _worlddirection 1000.0)) (`|MakeArray` "ObjectTypeQuery1" "ObjectTypeQuery2" "ObjectTypeQuery3" "ObjectTypeQuery4" "ObjectTypeQuery5" "ObjectTypeQuery6" :!type "EObjectTypeQuery Enum")))
  (return _outhit _returnvalue))